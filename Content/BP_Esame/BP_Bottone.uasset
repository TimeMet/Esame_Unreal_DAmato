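; BP_Bottone is a timed button that counts toward the BP_ThirdPersonGameMode Bottoni total while pressed.
; An actor overlap plays a timeline when inactive; on finish it lowers the Cube, increments Bottoni and sets Attivo.
; After a five-second delay it decrements the counter, clears Attivo and reverses a second timeline, whose update sets the Cube to its raised height with a fixed alpha.
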(event `self.ReceiveActorBeginOverlap`
  (params (OtherActor :type "Actor Object Reference"))
  (if (not (`self.Attivo`))
    (bind (_direction _altezza) (`Timeline|Timeline`)
      (:`Finished`
        (`SceneComponent.K2_SetRelativeLocation` (`self.Cube`) (`KismetMathLibrary.MakeVector` 0.0 0.0 (`KismetMathLibrary.Lerp` 3.0 -3.0 _altezza)) false false)
        (bind _asbp_third_person_game_mode (cast `/Game/ThirdPerson/Blueprints/BP_ThirdPersonGameMode` (`GameplayStatics.GetGameMode`)))
        (set `/Game/ThirdPerson/Blueprints/BP_ThirdPersonGameMode.Bottoni` (+ (`/Game/ThirdPerson/Blueprints/BP_ThirdPersonGameMode.Bottoni` _asbp_third_person_game_mode) 1) _asbp_third_person_game_mode)
        (set `self.Attivo` true)
        (`KismetSystemLibrary.PrintText` "+1")
        (`KismetSystemLibrary.Delay` 5.0)
        (bind _asbp_third_person_game_mode_2 (cast `/Game/ThirdPerson/Blueprints/BP_ThirdPersonGameMode` (`GameplayStatics.GetGameMode`)))
        (set `/Game/ThirdPerson/Blueprints/BP_ThirdPersonGameMode.Bottoni` (+ (`/Game/ThirdPerson/Blueprints/BP_ThirdPersonGameMode.Bottoni` _asbp_third_person_game_mode_2) -1) _asbp_third_person_game_mode_2)
        (set `self.Attivo` false)
        (`KismetSystemLibrary.PrintText` "-1")
        (`Timeline|Timeline_0` :!via `Reverse`
          (:`Update`
            (`SceneComponent.K2_SetRelativeLocation` (`self.Cube`) (`KismetMathLibrary.MakeVector` 0.0 0.0 (`KismetMathLibrary.Lerp` 3.0 -3.0)) false false)))))))

(fn `UserConstructionScript`)