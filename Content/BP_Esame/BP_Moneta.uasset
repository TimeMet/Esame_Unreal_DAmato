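; BP_Moneta is a pickup actor that acts as either a coin (Moneta) or a poison (Veleno), chosen by its Oggetto value.
; On BeginPlay it reads Punti from the matching row of the DT_Esame data table.
; When BP_ThirdPersonCharacter overlaps Sphere1, it passes Punti to the character's AddMoneta and destroys itself.
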(event `self.Sphere1.OnComponentBeginOverlap`
  (params (OverlappedComponent :type "PrimitiveComponent Object Reference") (OtherActor :type "Actor Object Reference") (OtherComp :type "PrimitiveComponent Object Reference") (OtherBodyIndex :type Integer) (bFromSweep :type Boolean) (SweepResult :type "HitResult Structure (by ref)"))
  (bind _asbp_third_person_character (cast `/Game/ThirdPerson/Blueprints/BP_ThirdPersonCharacter` OtherActor))
  (`/Game/ThirdPerson/Blueprints/BP_ThirdPersonCharacter.Add Moneta` _asbp_third_person_character (`self.Punti`))
  (`self.K2_DestroyActor`))

(event `self.ReceiveBeginPlay`
  (switch `/Game/BP_Esame/DTDA_Esame/E_Esame` (`self.Oggetto`)
    (:`NewEnumerator0`
      (bind _returnvalue (`|GetDataTableRow` "/Game/BP_Esame/DTDA_Esame/DT_Esame.DT_Esame" "Moneta")
        (:`then`
          (set `self.Punti` (`.Punti_11_98D51A304C52AA77203FE792E0A1B7AF` (break `/Game/BP_Esame/DTDA_Esame/ST_Esame` _returnvalue))))))
    (:`NewEnumerator1`
      (bind _returnvalue_2 (`|GetDataTableRow` "/Game/BP_Esame/DTDA_Esame/DT_Esame.DT_Esame" "Veleno")
        (:`then`
          (set `self.Punti` (`.Punti_11_98D51A304C52AA77203FE792E0A1B7AF` (break `/Game/BP_Esame/DTDA_Esame/ST_Esame` _returnvalue_2))))))))

(fn `UserConstructionScript`)