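; BP_TriggerBox is a one-shot trigger volume that counts when the player character enters it.
; On actor overlap by a BP_ThirdPersonCharacter, it increments the Counter on BP_ThirdPersonGameMode.
; A Triggered flag is then set so later overlaps with the same box do not count again.
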(event `self.ReceiveActorBeginOverlap`
  (params (OtherActor :type "Actor Object Reference"))
  (if (== (`GameplayStatics.GetObjectClass` OtherActor) "/Game/ThirdPerson/Blueprints/BP_ThirdPersonCharacter.BP_ThirdPersonCharacter_C")
    ; Se non ho ancora triggerato
    (if (not (`self.Triggered`))
      ; Aumento il counter
      (bind _asbp_third_person_game_mode (cast `/Game/ThirdPerson/Blueprints/BP_ThirdPersonGameMode` (`GameplayStatics.GetGameMode`)))
      (set `/Game/ThirdPerson/Blueprints/BP_ThirdPersonGameMode.Counter` (+ (`/Game/ThirdPerson/Blueprints/BP_ThirdPersonGameMode.Counter` _asbp_third_person_game_mode) 1) _asbp_third_person_game_mode)
      ; Triggero e non posso più farlo
      (set `self.Triggered` true))))

(fn `UserConstructionScript`)